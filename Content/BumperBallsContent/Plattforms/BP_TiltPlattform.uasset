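; Tilting platform for the Bumper Balls minigame that rotates toward new target rotations while a game runs.
; If visible when BP_PartyTimeGameMode signals start, it waits briefly, then repeatedly lerps toward targets from RandomFloatRange using Delay loops.
; Game end triggers an RInterpTo loop back to zero rotation, without explicitly stopping the tilt loop.
; CurrentRotation's OnRep applies rotation; an older authority-checked axis-picking graph is disconnected.
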(event `self.ReceiveBeginPlay`
  (bind _asbp_party_time_game_mode (cast `/Game/PartyTime/General/GameLogic/BP_PartyTimeGameMode` (`GameplayStatics.GetGameMode`)))
  (add `/Game/PartyTime/General/GameLogic/BP_PartyTimeGameMode.GameStartedDispatcher` _asbp_party_time_game_mode (delegate `GameStarted`)))

(event `TiltPlattform`
  (bind _returnvalue (`KismetMathLibrary.RLerp` (`self.K2_GetActorRotation`) (`self.CurrentRotationDestination`) 0.005))
  ;[1 1 1] Tilt the plattform randomly
  (set `self.CurrentRotationDestination` (`KismetMathLibrary.MakeRotator` (`self.RandomFloatRange`) (`self.RandomFloatRange`) (`self.RandomFloatRange`)))
  (set `self.CurrentRotation` _returnvalue :!label _label)
  (`self.K2_SetActorRotation` _returnvalue)
  (if (== (`self.K2_GetActorRotation`) (`self.CurrentRotationDestination`) :`ErrorTolerance` 1.0)
    (`KismetSystemLibrary.Delay` 0.5)
    (`self.TiltPlattform`)
    (else
      (`KismetSystemLibrary.Delay` 0.01)
      (goto _label))))

(event `GameStarted`
  (if (not (`self.bHidden`))
    (`|ExecutionSequence`
      (:`then_0`
        ;[1 1 1] When game finished -> rotate to default position
        (bind _asbp_party_time_game_mode (cast `/Game/PartyTime/General/GameLogic/BP_PartyTimeGameMode` (`GameplayStatics.GetGameMode`)))
        (add `/Game/PartyTime/General/GameLogic/BP_PartyTimeGameMode.GameEndedDispatcher` _asbp_party_time_game_mode (delegate `RotatePlattformToDefault`)))
      (:`then_1`
        (`KismetSystemLibrary.Delay` 3.0)
        (`self.TiltPlattform`)))))

(event `RotatePlattformToDefault`
  (bind _returnvalue (`self.K2_GetActorRotation`))
  (bind _returnvalue_2 (`KismetMathLibrary.RInterpTo` _returnvalue (struct) (`GameplayStatics.GetWorldDeltaSeconds`) 1.5))
  ;[1 1 1] When game finished -> rotate to default position
  (set `self.CurrentRotation` _returnvalue_2 :!label _label_2)
  (`self.K2_SetActorRotation` _returnvalue_2)
  (if (not (== _returnvalue (struct) :`ErrorTolerance` 0.5))
    (`KismetSystemLibrary.Delay` 0.001)
    (goto _label_2)))

(fn `OnRep_CurrentRotation`
  (`self.K2_SetActorRotation` (`self.CurrentRotation`)))

(fn `UserConstructionScript`)