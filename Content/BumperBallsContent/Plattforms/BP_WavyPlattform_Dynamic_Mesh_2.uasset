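; Wavy platform for Bumper Balls that animates a Geometry Script math warp on a dynamic mesh.
; The construction script copies InputMesh, tessellates it, sets collision and applies the warp.
; From BeginPlay, WarpPlattform loops on a tiny Delay, rebuilding mesh and collision each pass while the warp origin bounces along X.
; Magnitude interpolation is disconnected, though the near-limit check still toggles ReverseLerp.
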(event `self.ReceiveBeginPlay`
  (`self.WarpPlattform`))

(event `WarpPlattform`
  (bind _dynamicmeshcomponent (`self.DynamicMeshComponent`))
  (bind (_warporientation_location _warporientation_rotation _warporientation_scale) (`KismetMathLibrary.BreakTransform` (`self.WarpOrientation`)))
  ;[1 1 1] Interpolate and set wave magnitude
  (`|ExecutionSequence`
    (:`then_0`
      (`self.SetNewWaveOptions` (`self.GeometryScriptMathOptions`) (`self.WarpOrientation`) (`self.WarpType`)
        (:`Execution`
          (bind _returnvalue (`BaseDynamicMeshComponent.GetDynamicMesh` _dynamicmeshcomponent))
          (`GeometryScriptLibrary_CollisionFunctions.SetDynamicMeshCollisionFromMesh` _returnvalue _dynamicmeshcomponent (struct) null)
          (`KismetSystemLibrary.Delay` 0.001)
          (`self.CheckIfMagnitudeNearMinMax`)
          (`self.WarpPlattform`))))
    (:`then_1`
      (bind _output_get (set `self.WarpOrientation` (`KismetMathLibrary.MakeTransform` (+ _warporientation_location (`KismetMathLibrary.MakeVector` (* (`GameplayStatics.GetWorldDeltaSeconds`) (`self.XWarpOrientationSpeed`)))) _warporientation_rotation _warporientation_scale)))
      (bind _x (`KismetMathLibrary.BreakVector3f` (.location _output_get)))
      (if (> _x (`self.MaxXWarpOrientation`))
        (`/Engine/EditorBlueprintResources/StandardMacros.NegateFloat` (`self.XWarpOrientationSpeed`) :!label _label)
        (elif (< _x 0.0)
          (goto _label))))))

(event `CheckIfMagnitudeNearMinMax`
  (bind _maxmagnitude (`self.MaxMagnitude`))
  (bind _geometryscriptmathoptions_magnitude (break `GeometryScriptMathWarpOptions` (`self.GeometryScriptMathOptions`)))
  ;[1 1 1] Negate Speed if near min or max magnitude
  (bind _result_float (`self.NegateFloat` _maxmagnitude))
  (if (`KismetMathLibrary.NearlyEqual_FloatFloat` _geometryscriptmathoptions_magnitude _maxmagnitude 0.2)
    (set `self.ReverseLerp` (not (`self.ReverseLerp`)) :!label _label_2)
    (elif (`KismetMathLibrary.NearlyEqual_FloatFloat` _geometryscriptmathoptions_magnitude _result_float 0.2)
      (goto _label_2))))

(fn `NegateFloat`
  (params (Float :type "Float (double-precision)"))
  (returns (`Result Float` :type "Float (double-precision)"))
  (return (* Float -1.0)))

(fn `UserConstructionScript`
  (bind _returnvalue (`BaseDynamicMeshComponent.GetDynamicMesh` (`self.DynamicMeshComponent`)))
  (bind _returnvalue_2 (`GeometryScriptLibrary_StaticMeshFunctions.CopyMeshFromStaticMesh` (`self.InputMesh`) _returnvalue (struct) (struct) null)
    (:`Success`
      (bind _returnvalue_3 (`GeometryScriptLibrary_MeshSubdivideFunctions.ApplyUniformTessellation` _returnvalue_2 (`self.TesselationLevel`) null))
      (bind _returnvalue_4 (`GeometryScriptLibrary_CollisionFunctions.SetDynamicMeshCollisionFromMesh` _returnvalue_3 (`self.DynamicMeshComponent`) (struct) null))
      (`GeometryScriptLibrary_MeshDeformFunctions.ApplyMathWarpToMesh` _returnvalue_4 (`self.WarpOrientation`) (`self.WarpType`) (`self.GeometryScriptMathOptions`) null))))