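; Bumper Balls platform whose surface turns wavy during play and flattens again when the game ends.
; Geometry Script copies the input static mesh into a dynamic mesh, tessellates it and applies a math warp, in construction and every update.
; Five seconds after BeginPlay, a Delay-driven loop ramps wave magnitude toward its maximum while a cosine shifts the warp origin.
; The 4-player gamemode's game-ended dispatcher stops this loop and eases magnitude down.
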(event `self.ReceiveBeginPlay`
  (bind _asbp_4player_gamemode (cast `/Game/BumperBallsContent/PlayerScripts/BP_4Player_Gamemode` (`GameplayStatics.GetGameMode`)))
  (add `/Game/BumperBallsContent/PlayerScripts/BP_4Player_Gamemode.GameEndedDispatcher` _asbp_4player_gamemode (delegate `SmoothlyMakePlattformFlat`))
  (`KismetSystemLibrary.Delay` 5.0)
  (`self.WarpPlattform`))

(event `WarpPlattform`
  (bind (_geometryscriptmathoptions_magnitude _geometryscriptmathoptions_frequency _geometryscriptmathoptions_frequencyshift) (break `GeometryScriptMathWarpOptions` (`self.GeometryScriptMathOptions`)))
  (bind _warporientation (`self.WarpOrientation`))
  (bind _warptype (`self.WarpType`))
  (bind (_warporientation_location _warporientation_rotation _warporientation_scale) (`KismetMathLibrary.BreakTransform` (`self.WarpOrientation`)))
  ;[1 1 1] Interpolate and set wave magnitude
  (if (`self.MakePlattformWarp`)
    ;;[1 1 1] Increase WaveCosine
    (set `self.WaveCosine` (+ (`self.WaveCosine`) (* (`self.WaveCosineIncreaseAmount`) (`GameplayStatics.GetWorldDeltaSeconds`))))
    ;;[1 1 1] Set WaveCosine back to 0 if >= 360
    (if (>= (`self.WaveCosine`) 360.0)
      (set `self.WaveCosine` 0.0))
    (set `self.WarpOrientation` (`KismetMathLibrary.MakeTransform` (`KismetMathLibrary.MakeVector` (`KismetMathLibrary.Lerp` 0.0 (`self.TargetMaxMagnitude`) (`KismetMathLibrary.DegCos` (`self.WaveCosine`)))) _warporientation_rotation _warporientation_scale))
    (if (> _geometryscriptmathoptions_magnitude (`self.TargetMaxMagnitude`))
      (`self.SetNewWaveOptions` (`self.GeometryScriptMathOptions`) _warporientation _warptype
        (:`Execution`
          _))
      (else
        (bind _output_get (set `self.GeometryScriptMathOptions` (make `GeometryScriptMathWarpOptions` (+ _geometryscriptmathoptions_magnitude (* (`self.MagnitudeIncreaseAmount`) (`GameplayStatics.GetWorldDeltaSeconds`))) _geometryscriptmathoptions_frequency _geometryscriptmathoptions_frequencyshift)))
        (`self.SetNewWaveOptions` _output_get _warporientation _warptype
          (:`Execution`
            _))))
    (`KismetSystemLibrary.Delay` 0.001)
    (`self.WarpPlattform`)))

(event `SmoothlyMakePlattformFlat`
  (bind (_geometryscriptmathoptions_magnitude _geometryscriptmathoptions_frequency _geometryscriptmathoptions_frequencyshift) (break `GeometryScriptMathWarpOptions` (`self.GeometryScriptMathOptions`)))
  ;[1 1 1] Reset plattform to be flat again
  (set `self.MakePlattformWarp` false)
  (if (> _geometryscriptmathoptions_magnitude 0.0)
    (bind _output_get (set `self.GeometryScriptMathOptions` (make `GeometryScriptMathWarpOptions` (- _geometryscriptmathoptions_magnitude (* 15.0 (`GameplayStatics.GetWorldDeltaSeconds`))) _geometryscriptmathoptions_frequency _geometryscriptmathoptions_frequencyshift)))
    (`self.SetNewWaveOptions` _output_get (`self.WarpOrientation`) (`self.WarpType`)
      (:`Execution`
        (`KismetSystemLibrary.Delay` 0.001)
        (`self.SmoothlyMakePlattformFlat`)))))

(fn `NegateFloat`
  (params (Float :type "Float (double-precision)"))
  (returns (`Result Float` :type "Float (double-precision)"))
  (return (* Float -1.0)))

(fn `UserConstructionScript`
  (bind _returnvalue (`BaseDynamicMeshComponent.GetDynamicMesh` (`self.DynamicMeshComponent`)))
  (bind _returnvalue_2 (`GeometryScriptLibrary_StaticMeshFunctions.CopyMeshFromStaticMesh` (`self.InputMesh`) _returnvalue (struct) (struct) null)
    (:`Success`
      (bind _returnvalue_3 (`GeometryScriptLibrary_MeshSubdivideFunctions.ApplyUniformTessellation` _returnvalue_2 (`self.TesselationLevel`) null))
      (`GeometryScriptLibrary_MeshDeformFunctions.ApplyMathWarpToMesh` _returnvalue_3 (`self.WarpOrientation`) (`self.WarpType`) (`self.GeometryScriptMathOptions`) null))))