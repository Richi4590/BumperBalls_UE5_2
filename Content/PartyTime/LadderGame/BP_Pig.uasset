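; BP_Pig is an AI-moved pig for the LadderGame that wanders the navmesh.
; On BeginPlay a random coin flip may send it to a randomized first point along X, and reaching it starts the roaming cycle.
; The cycle alternates between trips to random navigable points and to a stored Destination, with random delays.
; Each trip uses AIMoveTo and records CurrentDestination.
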(event `self.ReceiveBeginPlay`
  (`self.MoveToTheFirstRandomPoint`))

(event `MoveToRandomPoint`
  (bind _randomlocation (`NavigationSystemV1.K2_GetRandomLocationInNavigableRadius` (`self.K2_GetActorLocation` self) 10000.0 null null))
  (`KismetSystemLibrary.Delay` (`KismetMathLibrary.RandomFloatInRange` 1.0 3.0))
  (bind _output_get (set `self.CurrentDestination` _randomlocation))
  (`|AIMoveTo` self _output_get null 5.0 true
    (:`then`
      _)
    (:`OnSuccess`
      _)
    (:`OnFail`
      _))
  (`self.MoveToDestination` true))

(event `MoveToDestination`
  (params (`Delay?` :type Boolean))
  (if `Delay?`
    (`KismetSystemLibrary.Delay` (`KismetMathLibrary.RandomFloatInRange` 5.0 10.0)))
  (bind _output_get (set `self.CurrentDestination` (`self.Destination`)))
  (bind _returnvalue (`NavigationSystemV1.FindPathToLocationSynchronously` (`self.K2_GetActorLocation` self) _output_get null null))
  (`|AIMoveTo` _returnvalue self (`self.CurrentDestination`) null 5.0 true
    (:`then`
      _)
    (:`OnSuccess`
      _)
    (:`OnFail`
      _))
  (`self.MoveToRandomPoint`))

(event `MoveToTheFirstRandomPoint`
  (if (`KismetMathLibrary.RandomBool`)
    (bind _result (`/Engine/EditorBlueprintResources/StandardMacros.NegateFloat` (`self.Multiplier`))
      (:`  `
        (set `self.Multiplier` _result)
        (`|AIMoveTo` self (`KismetMathLibrary.MakeVector` (* (`KismetMathLibrary.RandomFloatInRange` 2000.0 4000.0) (`self.Multiplier`)) 0.0 850.0) null 1000.0
          (:`OnSuccess`
            (`self.MoveToDestination` false)))))))

(fn `UserConstructionScript`)