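; BP_NavLink is a smart nav link that makes AI characters jump to the link's destination.
; When an agent reaches it, a Character is launched with a computed velocity, overriding its current XY and Z velocity.
; CalculateJumpVelocity derives that velocity from JumpDuration and hardcoded 981 gravity.
; Its Z term uses start minus destination height, the reverse of X and Y, so arcs only land correctly between equal heights.
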(event `self.ReceiveSmartLinkReached`
  (params (Agent :type "Actor Object Reference") (Destination :type "Vector Structure (by ref)"))
  (bind _ascharacter (cast `Character` Agent))
  (bind _velocity (`self.CalculateJumpVelocity` Destination (`self.K2_GetActorLocation` _ascharacter) (`self.JumpDuration`)))
  (`Character.LaunchCharacter` _ascharacter _velocity true true))

(fn `CalculateJumpVelocity`
  (params (Destination :type "Vector Structure") (Start :type "Vector Structure") (Duration :type "Float (double-precision)"))
  (returns (Velocity :type "Vector Structure"))
  (bind _induration (`self.InDuration`))
  (set `self.InDuration` Duration)
  (return (`KismetMathLibrary.MakeVector` (/ (- Destination_X Start_X) _induration) (/ (- Destination_Y Start_Y) _induration) (/ (- (+ Start_Z (* (`KismetMathLibrary.Square` (`self.InDuration`)) 0.5 981.0)) Destination_Z) _induration))))

(fn `UserConstructionScript`)