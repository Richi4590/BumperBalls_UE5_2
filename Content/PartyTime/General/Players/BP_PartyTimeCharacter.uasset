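; Networked wizard player character for Party Time, with a customizable outfit and an overhead name tag.
; EventReceived relays jump, taunt and outfit changes through server and multicast events; taunt only draws a debug point at the staff.
; Outfits recolor body and staff via dynamic materials and swap the staff mesh.
; The name's OnRep retries on a timer until the widget exists, and Tick turns the tag toward the local camera.
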(event `EventOnServer`
  (params (Event :type "/Game/PartyTime/General/GameLogic/Events Enum" :default "NewEnumerator0") (Outfit :type "/Game/PartyTime/General/Players/Outfit Structure"))
  ;[1 1 1] Event Handling
  (`self.EventMulticast` Event Outfit))

(event `EventMulticast`
  (params (Event :type "/Game/PartyTime/General/GameLogic/Events Enum" :default "NewEnumerator0") (Outfit :type "/Game/PartyTime/General/Players/Outfit Structure"))
  ;[1 1 1] Event Handling
  (`self.EventReceived` Event false Outfit))

(event `self.ReceiveBeginPlay`)

(event `EventReceived`
  (params (Event :type "/Game/PartyTime/General/GameLogic/Events Enum" :default "NewEnumerator0") (`OnServer?` :type Boolean) (Outfit :type "/Game/PartyTime/General/Players/Outfit Structure"))
  ;[1 1 1] Event Handling
  (if `OnServer?`
    (`self.EventOnServer` Event Outfit)
    (else
      (switch `/Game/PartyTime/General/GameLogic/Events` Event
        (:`NewEnumerator0`
          (`self.Jump`))
        (:`NewEnumerator1`
          (`self.Taunt`))
        (:`NewEnumerator2`
          (`self.SetUpPlayerOutfit` Outfit))))))

(event `SetPlayerNameOnServer`
  (params (CustomPlayerName :type Text))
  (set `self.CustomPlayerName` CustomPlayerName))

(event `self.ReceiveTick`
  (params (DeltaSeconds :type "Float (single-precision)"))
  (`self.CalculateDirectionForWidget`))

(fn `CalculateDirectionForWidget`
  (if (`self.IsLocallyControlled`)
    _
    (else
      _))
  (`SceneComponent.K2_SetWorldRotation` (`self.PlayerName`) (`KismetMathLibrary.FindLookAtRotation` (`SceneComponent.K2_GetComponentLocation` (`self.PlayerName`)) (`self.K2_GetActorLocation` (`GameplayStatics.GetPlayerCameraManager` 0))) false false))

(fn `OnRep_Clothes`)

(fn `OnRep_CurrentOutfit`)

(fn `OnRep_CustomPlayerName`
  (bind _returnvalue (`WidgetComponent.GetWidget` (`self.PlayerName`)))
  (`/Engine/EditorBlueprintResources/StandardMacros.IsValid` _returnvalue
    (:`Is Valid`
      (bind _asbp_player_name_tag (cast `/Game/PartyTime/General/Widgets/BP_PlayerNameTag` _returnvalue))
      (`/Game/PartyTime/General/Widgets/BP_PlayerNameTag.SetPlayerName` _asbp_player_name_tag (`self.CustomPlayerName`))
      (`SceneComponent.SetHiddenInGame` (`self.PlayerName`) false false))
    (:`Is Not Valid`
      (`KismetSystemLibrary.K2_SetTimer` null "OnRep_CustomPlayerName" 0.1))))

(fn `OnRep_isDead`)

(fn `SetClothes`
  (params (Outfit :type "/Game/PartyTime/General/Players/Outfit Structure"))
  (bind (_outfit_haircolor _outfit_outerclothescolor _outfit_innerclothcolor) (break `/Game/PartyTime/General/Players/Outfit` (`local.Outfit`)))
  (bind _outfit_haircolor_2 (break `/Game/PartyTime/General/Players/Outfit` (`local.Outfit`)))
  (bind (_outfit_haircolor_3 _outfit_outerclothescolor_2) (break `/Game/PartyTime/General/Players/Outfit` (`local.Outfit`)))
  (set `self.CurrentOutfit` Outfit)
  (bind _returnvalue (`KismetMaterialLibrary.CreateDynamicMaterialInstance` "/Game/BattleWizardPolyart/Materials/M_WizardColor.M_WizardColor"))
  (`MaterialInstanceDynamic.SetVectorParameterValue` _returnvalue "Hair" _outfit_haircolor_2)
  (`MaterialInstanceDynamic.SetVectorParameterValue` _returnvalue "OuterClothes" _outfit_outerclothescolor_2)
  (`MaterialInstanceDynamic.SetVectorParameterValue` _returnvalue "InnerCloth" _outfit_innerclothcolor)
  (`PrimitiveComponent.SetMaterial` (`self.Mesh`) 0 _returnvalue))

(fn `SetStaff`
  (params (Outfit :type "/Game/PartyTime/General/Players/Outfit Structure"))
  (bind (_outfit_haircolor _outfit_outerclothescolor _outfit_innerclothcolor) (break `/Game/PartyTime/General/Players/Outfit` (`local.Outfit`)))
  (bind _outfit_haircolor_2 (break `/Game/PartyTime/General/Players/Outfit` (`local.Outfit`)))
  (bind (_outfit_haircolor_3 _outfit_outerclothescolor_2) (break `/Game/PartyTime/General/Players/Outfit` (`local.Outfit`)))
  (bind _magicstaff (`self.MagicStaff`))
  (bind (_outfit_haircolor_4 _outfit_outerclothescolor_3 _outfit_innerclothcolor_2 _outfit_staff) (break `/Game/PartyTime/General/Players/Outfit` (`local.Outfit`)))
  (bind _returnvalue (`KismetMaterialLibrary.CreateDynamicMaterialInstance` "/Game/BattleWizardPolyart/Materials/M_WizardColor.M_WizardColor"))
  (`MaterialInstanceDynamic.SetVectorParameterValue` _returnvalue "Hair" _outfit_haircolor_2)
  (`MaterialInstanceDynamic.SetVectorParameterValue` _returnvalue "OuterClothes" _outfit_outerclothescolor_2)
  (`MaterialInstanceDynamic.SetVectorParameterValue` _returnvalue "InnerCloth" _outfit_innerclothcolor)
  (`StaticMeshComponent.SetStaticMesh` _magicstaff _outfit_staff)
  (`PrimitiveComponent.SetMaterial` _magicstaff 0 _returnvalue))

(fn `SetUpPlayerOutfit`
  (params (Outfit :type "/Game/PartyTime/General/Players/Outfit Structure"))
  (`self.SetClothes` Outfit)
  (`self.SetStaff` Outfit))

(fn `Taunt`
  (bind _returnvalue_location (`KismetMathLibrary.BreakTransform` (`SceneComponent.K2_GetComponentToWorld` (`self.MagicStaff`))))
  (`KismetSystemLibrary.DrawDebugPoint` _returnvalue_location 100.0 (struct :`R` 1.0 :`A` 1.0) 10.0))

(fn `UserConstructionScript`)