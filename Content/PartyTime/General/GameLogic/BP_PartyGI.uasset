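; BP_PartyGI, apparently the party game's Game Instance, keeps player data in a map keyed by PlayerController.
; SavePlayerLocally adds a controller's player record to the map.
; ChangePlayer moves a record from an old controller to a new one, rebuilding it with the new controller while keeping name, spectator flag, outfit and score, then returns it.
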(event `SavePlayerLocally`
  (params (PlayerController :type "/Game/PartyTime/General/GameLogic/BP_PartyTimePlayerController Object Reference") (Player :type "/Game/PartyTime/General/Players/Player Structure"))
  (`BlueprintMapLibrary.Map_Add` (`self.Players`) PlayerController Player))

(fn `Change Player`
  (params (OldPlayer :type "/Game/PartyTime/General/GameLogic/BP_PartyTimePlayerController Object Reference") (NewPlayer :type "/Game/PartyTime/General/GameLogic/BP_PartyTimePlayerController Object Reference"))
  (returns (Player :type "/Game/PartyTime/General/Players/Player Structure"))
  (locals (SavedPlayer :type "/Game/PartyTime/General/Players/Player Structure"))
  (bind _savedplayer (`local.SavedPlayer`))
  (bind _players (`self.Players`))
  (bind _value (`BlueprintMapLibrary.Map_Find` _players OldPlayer))
  (set `local.SavedPlayer` (make `/Game/PartyTime/General/Players/Player` NewPlayer (`.Name_15_5570C2C747A0D0628B0DFEA192C5D871` (break `/Game/PartyTime/General/Players/Player` _value)) (`.IsSpectator?_26_4E3196CA4ECD5E79F8432387A6B8E5B2` (break `/Game/PartyTime/General/Players/Player` _value)) (`.Outfit_5_F7CF110749F5AA9F61210AB7E8449EF0` (break `/Game/PartyTime/General/Players/Player` _value)) (`.Score_11_7026C0744903A64AA7BA3F800D51D201` (break `/Game/PartyTime/General/Players/Player` _value))))
  (`BlueprintMapLibrary.Map_Remove` _players (`local.OldPlayer`))
  (`BlueprintMapLibrary.Map_Remove` _players (`local.NewPlayer`))
  (`BlueprintMapLibrary.Map_Add` _players (`local.NewPlayer`) _savedplayer)
  (return _savedplayer))