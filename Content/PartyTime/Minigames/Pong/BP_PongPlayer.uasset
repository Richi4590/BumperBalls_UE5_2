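; Player pawn for the Pong party minigame: a paddle that slides along its right axis and has its own goal.
; MoveRight input moves it along the right vector cached from the capsule at BeginPlay.
; Balls overlapping the Goal report on the server to the Pong game mode's ScoreChanged with this player's controller.
; Paddle hits slightly speed up the ball and flatten its Z velocity, with a DoOnce and short delay debouncing repeats.
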(event `self.ReceiveBeginPlay`
  (`parent.ReceiveBeginPlay`)
  (set `self.Right` (`SceneComponent.GetRightVector` (`self.CapsuleComponent`))))

(event `InputAxis|MoveRight` :overrideparent false
  (params (AxisValue :type "Float (single-precision)"))
  (bind _output_get (set `self.Speed` AxisValue))
  (`self.AddMovementInput` (`self.Right`) _output_get))

(event `self.Goal.OnComponentBeginOverlap`
  (params (OverlappedComponent :type "PrimitiveComponent Object Reference") (OtherActor :type "Actor Object Reference") (OtherComp :type "PrimitiveComponent Object Reference") (OtherBodyIndex :type Integer) (bFromSweep :type Boolean) (SweepResult :type "HitResult Structure (by ref)"))
  (`/Engine/EditorBlueprintResources/ActorMacros.Switch Has Authority`
    (:`Authority`
      (bind _asbp_pong_ball (cast `/Game/PartyTime/Minigames/Pong/BP_PongBall` OtherActor))
      (bind _asbp_party_time_game_mode_pong (cast `/Game/PartyTime/Minigames/Pong/BP_PartyTimeGameModePong` (`GameplayStatics.GetGameMode`)))
      (bind _asbp_party_time_player_controller (cast `/Game/PartyTime/General/GameLogic/BP_PartyTimePlayerController` (`self.GetController`)))
      (`/Game/PartyTime/Minigames/Pong/BP_PartyTimeGameModePong.ScoreChanged` _asbp_party_time_game_mode_pong _asbp_party_time_player_controller _asbp_pong_ball))))

(event `self.Paddle.OnComponentHit`
  (params (HitComponent :type "PrimitiveComponent Object Reference") (OtherActor :type "Actor Object Reference") (OtherComp :type "PrimitiveComponent Object Reference") (NormalImpulse :type "Vector Structure") (Hit :type "HitResult Structure (by ref)"))
  ;[1 1 1] OnHit Bounce Player and Play Sound
  (`/Engine/EditorBlueprintResources/StandardMacros.DoOnce` false :!label _label
    (:`Completed`
      (bind _asbp_pong_ball (cast `/Game/PartyTime/Minigames/Pong/BP_PongBall` OtherActor))
      (`KismetSystemLibrary.PrintString` "Paddle Hit!")
      (if (`KismetSystemLibrary.IsValid` _asbp_pong_ball)
        (bind (_returnvalue_x _returnvalue_y) (`KismetMathLibrary.BreakVector` (* (`MovementComponent.Velocity` (`/Game/PartyTime/Minigames/Pong/BP_PongBall.ProjectileMovement` _asbp_pong_ball)) 1.05)))
        (set `/Game/PartyTime/Minigames/Pong/BP_PongBall.Velocity` (`KismetMathLibrary.MakeVector` (+ _returnvalue_x 0.0) (+ _returnvalue_y 0.0)) _asbp_pong_ball)
        (`KismetSystemLibrary.Delay` 0.1)
        (goto _label :!via `Reset`)))))

(fn `UserConstructionScript`
  (`parent.UserConstructionScript`))