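; BP_PongBall is the ball for the Pong minigame, driven by a ProjectileMovement component.
; On BeginPlay the server sets a fixed negative-Y launch through AddVelocity, and Velocity's RepNotify copies it into the movement component.
; The bounce handler's randomized velocity rewrite is effectively unreachable, since it needs a successful ball cast that is also invalid.
; Tick prints velocity for debugging, and a random diagonal launch is left unconnected.
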(event `self.ReceiveBeginPlay`
  (`/Engine/EditorBlueprintResources/ActorMacros.Switch Has Authority`
    (:`Authority`
      (`self.AddVelocity` 0.0 0.0 -1000.0 -1000.0))))

(event `self.ProjectileMovement.OnProjectileBounce`
  (params (ImpactResult :type "HitResult Structure (by ref)") (ImpactVelocity :type "Vector Structure (by ref)"))
  (bind _returnvalue (`KismetMathLibrary.RandomFloatInRange` 0.7 1.3))
  (bind (_returnvalue_x _returnvalue_y) (`KismetMathLibrary.BreakVector` (`KismetMathLibrary.ClampVectorSize` (`MovementComponent.Velocity` (`self.ProjectileMovement`)))))
  (bind _asbp_pong_ball (cast `/Game/PartyTime/Minigames/Pong/BP_PongBall` ImpactResult_HitActor))
  (if (not (`KismetSystemLibrary.IsValid` _asbp_pong_ball))
    (set `self.Velocity` (`KismetMathLibrary.MakeVector` (+ _returnvalue_x _returnvalue) (+ _returnvalue_y _returnvalue)))))

(event `self.ReceiveTick`
  (params (DeltaSeconds :type "Float (single-precision)"))
  (`KismetSystemLibrary.PrintString` (`KismetStringLibrary.Conv_VectorToString` (`MovementComponent.Velocity` (`self.ProjectileMovement`)))))

(fn `OnRep_Velocity`
  (set `MovementComponent.Velocity` (`self.Velocity`) (`self.ProjectileMovement`)))

(fn `UserConstructionScript`)