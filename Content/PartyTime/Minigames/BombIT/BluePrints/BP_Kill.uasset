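; Short-lived damage volume for the BombIT minigame that applies kill effects to whatever actor begins overlapping it.
; On BeginPlay it takes its lifespan from the level manager's LifeOfKill.
; A cast chain on overlap removes a life from players, calls DonateBomb on bombs, destroys bubbles, and calls DestroyWall on breakable walls with a delay derived from its own lifespan.
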(event `self.ReceiveBeginPlay`
  (bind _returnvalue (`GameplayStatics.GetActorOfClass` "/Game/PartyTime/Minigames/BombIT/BluePrints/Core/BP_LevelManager.BP_LevelManager_C"))
  (`self.SetLifeSpan` (`/Game/PartyTime/Minigames/BombIT/BluePrints/Core/BP_LevelManager.LifeOfKill` _returnvalue)))

(event `self.ReceiveActorBeginOverlap`
  (params (OtherActor :type "Actor Object Reference"))
  (bind _asbp_bomb_player (cast `/Game/PartyTime/Minigames/BombIT/BluePrints/BP_BombPlayer` OtherActor)
    (:`then`
      (`/Game/PartyTime/Minigames/BombIT/BluePrints/BP_BombPlayer.Reduce Life Client` _asbp_bomb_player 1))
    (:`CastFailed`
      (bind _asbp_bomb (cast `/Game/PartyTime/Minigames/BombIT/BluePrints/BP_Bomb` OtherActor)
        (:`then`
          (`/Game/PartyTime/Minigames/BombIT/BluePrints/BP_Bomb.DonateBomb` _asbp_bomb))
        (:`CastFailed`
          (bind _asbp_bubble (cast `/Game/PartyTime/Minigames/BombIT/BluePrints/Bubbles/BP_Bubble` OtherActor)
            (:`then`
              (`self.K2_DestroyActor` _asbp_bubble))
            (:`CastFailed`
              (bind _asbp_breakable_wall (cast `/Game/PartyTime/Minigames/BombIT/BluePrints/Environment/Wall/BP_BreakableWall` OtherActor))
              (`/Game/PartyTime/Minigames/BombIT/BluePrints/Environment/Wall/BP_BreakableWall.Destroy Wall` _asbp_breakable_wall (+ (`self.GetLifeSpan`) 0.5)))))))))

(fn `UserConstructionScript`)