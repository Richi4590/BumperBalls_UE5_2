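; BP_ExplosionManager creates a cross-shaped, grid-aligned bomb explosion for the BombIT minigame.
; On BeginPlay, the server spawns a BP_Kill at its location and runs OneLineKill along forward, back, right and left.
; Each arm line-traces using BP_LevelManager's grid sizes, spawning BP_Kill per tile up to BombRadius or the blocking wall.
; Breakable walls receive an extra BP_Kill one tile further.
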(event `self.ReceiveBeginPlay`
  (bind _returnvalue (`self.K2_GetActorLocation`))
  (bind _returnvalue_2 (`self.GetActorForwardVector`))
  (bind _returnvalue_3 (`self.GetActorRightVector`))
  (bind _bombradius (`self.BombRadius`))
  (if (`KismetSystemLibrary.IsServer`)
    (`self.OneLineKill` _bombradius _returnvalue _returnvalue_2)
    (`self.OneLineKill` _bombradius _returnvalue (* _returnvalue_2 -1))
    (`self.OneLineKill` _bombradius _returnvalue _returnvalue_3)
    (`self.OneLineKill` _bombradius _returnvalue (* _returnvalue_3 -1))
    (`|SpawnActorFromClass` "/Game/PartyTime/Minigames/BombIT/BluePrints/BP_Kill.BP_Kill_C" (`KismetMathLibrary.MakeTransform` _returnvalue) "Undefined" "MultiplyWithRoot" null null)))

(fn `OneLineKill`
  (params (Radius :type Integer) (StartLocation :type "Vector Structure") (Direction :type "Vector Structure"))
  (bind _returnvalue (`GameplayStatics.GetActorOfClass` "/Game/PartyTime/Minigames/BombIT/BluePrints/Core/BP_LevelManager.BP_LevelManager_C"))
  (bind _outhit (`KismetSystemLibrary.LineTraceSingleForObjects` StartLocation (+ StartLocation (* Direction (* (`/Game/PartyTime/Minigames/BombIT/BluePrints/Core/BP_LevelManager.DefaultLineLength` _returnvalue) (+ Radius 0.5)))) (`|MakeArray` "ObjectTypeQuery1" :!type "EObjectTypeQuery Enum")))
  (bind (_bblockinghit _binitialoverlap _time _distance _location _impactpoint _normal _impactnormal _physmat _hitactor) (`GameplayStatics.BreakHitResult` _outhit))
  (if _bblockinghit
    (if (`GameplayStatics.ObjectIsA` _hitactor "/Game/PartyTime/Minigames/BombIT/BluePrints/Environment/Wall/BP_Wall.BP_Wall_C")
      (bind _floorsize (`/Game/PartyTime/Minigames/BombIT/BluePrints/Core/BP_LevelManager.FloorSize` _returnvalue))
      (bind (_remainder _returnvalue_2) (`KismetMathLibrary.FMod` _distance (`KismetMathLibrary.Conv_IntToDouble` _floorsize)))
      (for _index (range 1 (+ _returnvalue_2 1))
        (bind _returnvalue_3 (* _floorsize Direction))
        (`|SpawnActorFromClass` "/Game/PartyTime/Minigames/BombIT/BluePrints/BP_Kill.BP_Kill_C" (`KismetMathLibrary.MakeTransform` (+ (* _index _returnvalue_3) StartLocation)) "Undefined" "MultiplyWithRoot" null null))
      (if (`GameplayStatics.ObjectIsA` _hitactor "/Game/PartyTime/Minigames/BombIT/BluePrints/Environment/Wall/BP_BreakableWall.BP_BreakableWall_C")
        (`|SpawnActorFromClass` "/Game/PartyTime/Minigames/BombIT/BluePrints/BP_Kill.BP_Kill_C" (`KismetMathLibrary.MakeTransform` (+ (* (+ _returnvalue_2 1) _returnvalue_3) StartLocation)) "Undefined" "MultiplyWithRoot" null null)))
    (else
      (for _index_2 (range 1 (+ Radius 1))
        (`|SpawnActorFromClass` "/Game/PartyTime/Minigames/BombIT/BluePrints/BP_Kill.BP_Kill_C" (`KismetMathLibrary.MakeTransform` (+ (* _index_2 _returnvalue_3) StartLocation)) "Undefined" "MultiplyWithRoot" null null)))))

(fn `UserConstructionScript`)