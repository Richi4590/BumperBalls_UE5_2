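; BP_Bomb is the placeable bomb in the BombIT minigame, exploding when its fuse delay runs out.
; DonateBomb runs once, refunding a bomb to its owner up to their maximum, spawning BP_ExplosionManager with the bomb's radius, then destroying the actor.
; The collider starts without collision and becomes physical when a player leaves the overlap listener.
; That listener also blocks bomb placement while a player is inside.
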(event `self.ReceiveBeginPlay`
  ;[1 1 1] Bomb explodes
  (`KismetSystemLibrary.Delay` (`self.BombLife`))
  (`self.DonateBomb`))

(event `self.OverlapListener.OnComponentEndOverlap`
  (params (OverlappedComponent :type "PrimitiveComponent Object Reference") (OtherActor :type "Actor Object Reference") (OtherComp :type "PrimitiveComponent Object Reference") (OtherBodyIndex :type Integer))
  ;[1 1 1] Make bomb physical
  (bind _asbp_bomb_player (cast `/Game/PartyTime/Minigames/BombIT/BluePrints/BP_BombPlayer` OtherActor))
  (`PrimitiveComponent.SetCollisionEnabled` (`self.Collider`) "QueryAndPhysics")
  (set `/Game/PartyTime/Minigames/BombIT/BluePrints/BP_BombPlayer.CanPlaceBomb` true _asbp_bomb_player))

(event `self.OverlapListener.OnComponentBeginOverlap`
  (params (OverlappedComponent :type "PrimitiveComponent Object Reference") (OtherActor :type "Actor Object Reference") (OtherComp :type "PrimitiveComponent Object Reference") (OtherBodyIndex :type Integer) (bFromSweep :type Boolean) (SweepResult :type "HitResult Structure (by ref)"))
  ;[1 1 1] Stop player placing bombs while he is inside it
  (bind _asbp_bomb_player (cast `/Game/PartyTime/Minigames/BombIT/BluePrints/BP_BombPlayer` OtherActor))
  (set `/Game/PartyTime/Minigames/BombIT/BluePrints/BP_BombPlayer.CanPlaceBomb` false _asbp_bomb_player))

(fn `DonateBomb`
  (bind _bombowner (`self.BombOwner`))
  (bind _bombamount (`/Game/PartyTime/Minigames/BombIT/BluePrints/BP_BombPlayer.BombAmount` _bombowner))
  (if (not (`self.Exploded`))
    (set `self.Exploded` true)
    (if (`KismetSystemLibrary.IsValid` _bombowner)
      (if (< _bombamount (`/Game/PartyTime/Minigames/BombIT/BluePrints/BP_BombPlayer.MaxBombs` _bombowner))
        (set `/Game/PartyTime/Minigames/BombIT/BluePrints/BP_BombPlayer.BombAmount` (+ _bombamount 1) _bombowner)))
    (`|SpawnActorFromClass` "/Game/PartyTime/Minigames/BombIT/BluePrints/BP_ExplosionManager.BP_ExplosionManager_C" (`self.GetTransform`) "Undefined" "MultiplyWithRoot" null (`self.BombRadius`) null)
    (`self.K2_DestroyActor`)))

(fn `UserConstructionScript`
  (`PrimitiveComponent.SetCollisionEnabled` (`self.Collider`) "NoCollision"))