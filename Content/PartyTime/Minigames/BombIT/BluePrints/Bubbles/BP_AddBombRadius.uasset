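; Pickup bubble in the BombIT minigame that increases a player's bomb blast radius.
; When a BP_BombPlayer overlaps it, the bubble adds one to that player's BombRadius and calls NotifyStatsChanged.
; It then destroys itself; other overlapping actors are ignored.
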(event `self.ReceiveActorBeginOverlap`
  (params (OtherActor :type "Actor Object Reference"))
  (bind _asbp_bomb_player (cast `/Game/PartyTime/Minigames/BombIT/BluePrints/BP_BombPlayer` OtherActor))
  (set `/Game/PartyTime/Minigames/BombIT/BluePrints/BP_BombPlayer.BombRadius` (+ (`/Game/PartyTime/Minigames/BombIT/BluePrints/BP_BombPlayer.BombRadius` _asbp_bomb_player) 1) _asbp_bomb_player)
  (`self.NotifyStatsChanged`)
  (`self.K2_DestroyActor`))

(fn `UserConstructionScript`
  (`parent.UserConstructionScript`))