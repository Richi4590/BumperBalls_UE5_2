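; BP_BubbleGenerator is a one-shot spawner for power-up bubbles in the BombIT minigame.
; On BeginPlay it waits a configurable delay, spawns a bubble at its own transform, then destroys itself.
; Type selects a bomb, life, speed or bomb radius bubble, or a random roll across them.
; The random roll includes zero, which has no case, so it can spawn nothing.
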(event `self.ReceiveBeginPlay`
  (`KismetSystemLibrary.Delay` (`self.Delay`))
  (`self.Generate Bubble`)
  (`self.K2_DestroyActor`))

(fn `Generate Bubble`
  (locals (RandomNumber :type Integer :default 0))
  (bind _returnvalue (`self.GetTransform`))
  (switch `/Game/MyThings/Enum/E_Bubbles` (`self.Type`)
    (:`NewEnumerator0`
      (bind _output_get (set `local.RandomNumber` (`KismetMathLibrary.RandomInteger` (+ (`self.NumberOfSpecialBubbles`) 1))))
      (switch `int` _output_get
        (:`1`
          (`|SpawnActorFromClass` "/Game/PartyTime/Minigames/BombIT/BluePrints/Bubbles/BP_AddBomb.BP_AddBomb_C" _returnvalue "Undefined" "MultiplyWithRoot" null null :!label _label))
        (:`2`
          (`|SpawnActorFromClass` "/Game/PartyTime/Minigames/BombIT/BluePrints/Bubbles/BP_AddLife.BP_AddLife_C" _returnvalue "Undefined" "MultiplyWithRoot" null null :!label _label_2))
        (:`3`
          (`|SpawnActorFromClass` "/Game/PartyTime/Minigames/BombIT/BluePrints/Bubbles/BP_AddSpeed.BP_AddSpeed_C" _returnvalue "Undefined" "MultiplyWithRoot" null null :!label _label_3))
        (:`4`
          (`|SpawnActorFromClass` "/Game/PartyTime/Minigames/BombIT/BluePrints/Bubbles/BP_AddBombRadius.BP_AddBombRadius_C" _returnvalue "Undefined" "MultiplyWithRoot" null null :!label _label_4))))
    (:`NewEnumerator3`
      (goto _label))
    (:`NewEnumerator2`
      (goto _label_2))
    (:`NewEnumerator4`
      (goto _label_3))
    (:`NewEnumerator5`
      (goto _label_4))))

(fn `UserConstructionScript`)