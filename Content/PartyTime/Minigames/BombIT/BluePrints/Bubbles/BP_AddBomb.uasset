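; BP_AddBomb is a bubble pickup in the BombIT minigame that grants an extra bomb to a BP_BombPlayer that overlaps it.
; On overlap it raises the player's MaxBombs by one, then compares BombAmount against that new maximum plus one.
; If BombAmount is lower, it increments BombAmount, calls NotifyStatsChanged and destroys itself; otherwise the pickup stays in place.
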(event `self.ReceiveActorBeginOverlap`
  (params (OtherActor :type "Actor Object Reference"))
  (bind _asbp_bomb_player (cast `/Game/PartyTime/Minigames/BombIT/BluePrints/BP_BombPlayer` OtherActor))
  (bind _returnvalue (+ (`/Game/PartyTime/Minigames/BombIT/BluePrints/BP_BombPlayer.MaxBombs` _asbp_bomb_player) 1))
  (set `/Game/PartyTime/Minigames/BombIT/BluePrints/BP_BombPlayer.MaxBombs` _returnvalue _asbp_bomb_player)
  (bind _bombamount (`/Game/PartyTime/Minigames/BombIT/BluePrints/BP_BombPlayer.BombAmount` _asbp_bomb_player))
  (if (< _bombamount _returnvalue)
    (set `/Game/PartyTime/Minigames/BombIT/BluePrints/BP_BombPlayer.BombAmount` (+ _bombamount 1) _asbp_bomb_player)
    (`self.NotifyStatsChanged`)
    (`self.K2_DestroyActor`)))

(fn `UserConstructionScript`)