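; BP_BreakableWall is a destructible wall for the BombIT minigame.
; Its DestroyWall event optionally spawns a BP_BubbleGenerator at the wall's transform, gated by CreateBubble, then destroys the wall immediately.
; The spawned generator receives the event's Delay and the wall's BubbleType, so the delay applies to the generator rather than to the wall's removal.
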(event `Destroy Wall`
  (params (Delay :type "Float (double-precision)"))
  (if (`self.CreateBubble`)
    (`|SpawnActorFromClass` "/Game/PartyTime/Minigames/BombIT/BluePrints/Bubbles/BP_BubbleGenerator.BP_BubbleGenerator_C" (`self.GetTransform`) "Undefined" "MultiplyWithRoot" null Delay (`self.BubbleType`) null))
  (`self.K2_DestroyActor`))

(fn `UserConstructionScript`
  (`parent.UserConstructionScript`))