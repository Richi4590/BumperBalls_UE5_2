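; Game mode for the Party Time racing minigame, which sets up the maze and two-player cart teams once all players arrive.
; The server builds an odd-sized labyrinth from a random seed and sends seed and size to each non-spectator player's controller.
; It then shuffles players with a retry-based random picker and pairs four as driver and partner on two carts, without waiting for maze-ready events, whose handlers are empty.
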(event `self.ReceiveTick`
  (params (DeltaSeconds :type "Float (single-precision)")))

(event `self.ReceiveBeginPlay`
  (`parent.ReceiveBeginPlay`)
  (add `self.AllPlayersArrivedDispatcher` (delegate `AllPlayersArrived`))
  (add `self.MazeReadyClientDispatcher` (delegate `MazeClientReady`))
  (add `self.MazeReadyServerDispatcher` (delegate `MazeServerReady`)))

(event `MazeClientReady`)

(event `MazeServerReady`)

(event `AllPlayersArrived`
  (bind _outactors (`GameplayStatics.GetAllActorsOfClass` "/Game/PartyTime/Minigames/RacingGame/Maze/BP_Maze.BP_Maze_C"))
  (for _array_element _outactors
    ;[1 1 1] Generate a randomly sized labyrinth
    (bind _output_get (set `self.size` (`KismetMathLibrary.RandomIntegerInRange` 11 11)))
    (if (== (mod _output_get 2) 0)
      (bind _seedout (`/Game/PartyTime/Minigames/RacingGame/Maze/BP_Maze.CreateNewLabyrinth` _array_element _array_element true 0 (+ _output_get 1)))
      (set `self.seed` _seedout)
      (`/Game/PartyTime/Minigames/RacingGame/Maze/BP_Maze.BuildLabyrinth` _array_element true)
      (else
        (bind _seedout_2 (`/Game/PartyTime/Minigames/RacingGame/Maze/BP_Maze.CreateNewLabyrinth` _array_element _array_element true 0 _output_get))
        (set `self.seed` _seedout_2)
        (`/Game/PartyTime/Minigames/RacingGame/Maze/BP_Maze.BuildLabyrinth` _array_element true))))
  ;[1 1 1] Send built maze info from server to all clients
  (bind _player (`self.ForEveryPhysicalPlayer`)
    (:`Iteration`
      (`/Game/PartyTime/General/GameLogic/BP_PartyTimePlayerController.RetrieveLabyrinthInfo` (break `/Game/PartyTime/General/Players/Player` _player) (`self.seed`) (`self.size`)))
    (:`Completed`
      ;[1 1 1] Clients done with building maze -> assign them randomly in pairs
      (bind _randomarray (`self.RandomizePlayers`))
      (bind _outactors_2 (`GameplayStatics.GetAllActorsOfClass` "/Game/PartyTime/Minigames/RacingGame/VehicleTemplate/Blueprints/RacingCart/RacingCart_Pawn.RacingCart_Pawn_C"))
      (bind _output (`|GetArrayItem` _randomarray))
      (bind _output_2 (`|GetArrayItem` _randomarray 1))
      (bind _output_3 (`|GetArrayItem` _outactors_2))
      (`/Game/PartyTime/General/GameLogic/BP_PartyTimePlayerController.SetPartner` _output _output_2 _output_3 true)
      (`/Game/PartyTime/General/GameLogic/BP_PartyTimePlayerController.SetPartner` _output_2 _output _output_3 false)
      (bind _output_4 (`|GetArrayItem` _randomarray 2))
      (bind _output_5 (`|GetArrayItem` _randomarray 3))
      (bind _output_6 (`|GetArrayItem` _outactors_2 1))
      (`/Game/PartyTime/General/GameLogic/BP_PartyTimePlayerController.SetPartner` _output_4 _output_5 _output_6 true)
      (`/Game/PartyTime/General/GameLogic/BP_PartyTimePlayerController.SetPartner` _output_5 _output_4 _output_6 false))))

(fn `RandomizePlayers`
  (returns (RandomArray :type "Array of /Game/PartyTime/General/GameLogic/BP_PartyTimePlayerController Object Reference"))
  (locals (TempArray :type "Array of /Game/PartyTime/General/GameLogic/BP_PartyTimePlayerController Object Reference") (RandomPlayerArray :type "Array of /Game/PartyTime/General/GameLogic/BP_PartyTimePlayerController Object Reference") (UsedIndexesArray :type "Array of Integer"))
  (bind _temparray (`local.TempArray`))
  (bind _values (`BlueprintMapLibrary.Map_Values` (`self.Players`)))
  (for _array_element _values
    (if (not (`.IsSpectator?_26_4E3196CA4ECD5E79F8432387A6B8E5B2` (break `/Game/PartyTime/General/Players/Player` _array_element)))
      (`KismetArrayLibrary.Array_Add` (`local.TempArray`) (break `/Game/PartyTime/General/Players/Player` _array_element))))
  (for _ _temparray
    (bind _wildcard (`self.GetRandomArrayIndex` _temparray (`local.UsedIndexesArray`) :!label _label)
      (:`Execution`
        (`KismetArrayLibrary.Array_Add` (`local.RandomPlayerArray`) _wildcard))
      (:`Redo`
        (goto _label))))
  (return (`local.RandomPlayerArray`)))

(fn `UserConstructionScript`
  (`parent.UserConstructionScript`))