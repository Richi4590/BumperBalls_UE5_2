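; Catapult actor for the WiiTanks part of PartyTime that plays a replicated firing animation with particles.
; LaunchPlayer routes through server and multicast events, then Launch and Retreat timelines swing the arm's roll out and back, with a DoOnce blocking refires until done.
; Sphere overlaps set a PlayerNearby flag after a character class cast, but nothing here reads it or applies launch force.
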(event `self.ReceiveTick`
  (params (DeltaSeconds :type "Float (single-precision)")))

(event `self.Sphere.OnComponentBeginOverlap`
  (params (OverlappedComponent :type "PrimitiveComponent Object Reference") (OtherActor :type "Actor Object Reference") (OtherComp :type "PrimitiveComponent Object Reference") (OtherBodyIndex :type Integer) (bFromSweep :type Boolean) (SweepResult :type "HitResult Structure (by ref)"))
  (`self.SetPlayerNearby` OtherActor true))

(event `self.Sphere.OnComponentEndOverlap`
  (params (OverlappedComponent :type "PrimitiveComponent Object Reference") (OtherActor :type "Actor Object Reference") (OtherComp :type "PrimitiveComponent Object Reference") (OtherBodyIndex :type Integer))
  (`self.SetPlayerNearby` OtherActor))

(event `Taunt_Multicast`)

(event `LaunchPlayer`
  ;[1 1 1] Shoot
  (`self.Launch(Server)`))

(event `Launch(Server)`
  ;[1 1 1] Shoot
  (`self.Launch(Multicast)`))

(event `Launch(Multicast)`
  ;[1 1 1] Shoot
  (`self.LaunchCatapult`))

(event `LaunchCatapult`
  ;[1 1 1] Shoot
  (`/Engine/EditorBlueprintResources/StandardMacros.DoOnce` false :!label _label
    (:`Completed`
      (`ActorComponent.Activate` (`self.ParticleSystem`) false)
      (bind (_direction _shoot) (`Timeline|Launch` :!via `PlayFromStart`)
        (:`Update`
          (`SceneComponent.K2_SetRelativeRotation` (`self.Catapult`) (`KismetMathLibrary.MakeRotator` _shoot) false false))
        (:`Finished`
          (`ActorComponent.Deactivate` (`self.ParticleSystem`))
          (bind (_direction_2 _shoot_2) (`Timeline|Retreat` :!via `ReverseFromEnd`)
            (:`Update`
              (`SceneComponent.K2_SetRelativeRotation` (`self.Catapult`) (`KismetMathLibrary.MakeRotator` _shoot_2) false false))
            (:`Finished`
              (goto _label :!via `Reset`))))))))

(fn `UserConstructionScript`)